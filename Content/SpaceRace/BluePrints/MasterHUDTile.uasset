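; MasterHUDTile is a track tile Blueprint for endless, chained level spawning in the SpaceRace flying game.
; When a FlyingPawn enters its collision box, it passes a transform to FlyingGameMode and calls SpawnTile.
; That transform combines the SpawnPoint component's location with the tile root's rotation and scale.
; The tile destroys itself ten seconds after any overlap with the box ends, without checking the actor type.
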(event OnComponentBeginOverlap(Box_Collision)
  (params (OverlappedComponent :type Primitive%20Component%20Object%20Reference) (OtherActor :type Actor%20Object%20Reference) (OtherComp :type Primitive%20Component%20Object%20Reference) (OtherBodyIndex :type Integer) (bFromSweep :type Boolean) (SweepResult :type Hit%20Result%20Structure%20%28by%20ref%29))
  (bind _defaultsceneroot (Variables|Default|GetDefaultSceneRoot))
  (bind _returnvalue (Transformation|GetWorldTransform _defaultsceneroot))
  (bind (_location _rotation _scale) (Math|Transform|BreakTransform _returnvalue))
  (bind _output_get (Variables|Default|SetNextSpawnPoint (Math|Transform|MakeTransform (Transformation|GetWorldLocation (Variables|Default|GetSpawnPoint)) _rotation _scale)))
  (Utilities|Casting|CastToFlyingPawn OtherActor)
  (bind _asflying_game_mode (Utilities|Casting|CastToFlyingGameMode (Game|GetGameMode)))
  (Variables|/Game/FlyingBP/Blueprints/FlyingGameMode.FlyingGameMode_C|SetNextSpawnPoint _asflying_game_mode _output_get)
  (Default|SpawnTile _asflying_game_mode))

(event OnComponentEndOverlap(Box_Collision)
  (params (OverlappedComponent :type Primitive%20Component%20Object%20Reference) (OtherActor :type Actor%20Object%20Reference) (OtherComp :type Primitive%20Component%20Object%20Reference) (OtherBodyIndex :type Integer))
  (Utilities|FlowControl|Delay 1e+01)
  (Actor|DestroyActor))

(fn ConstructionScript)