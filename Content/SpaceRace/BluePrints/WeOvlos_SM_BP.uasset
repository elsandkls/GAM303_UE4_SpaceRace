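; WeOvlos_SM_BP is a SpaceRace Blueprint that plays animal sounds while it hovers.
; Tick polls the HoverStatus of its Hover component, starting and fading in the AnimalSounds audio when hovering begins.
; While not hovering, it calls FadeOut every tick the audio is playing, targeting the fade-in's volume level rather than silence.
; BeginPlay, overlap, physics-volume events and the construction script are empty.
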(event PhysicsVolumeChangedDelegate(AnimalSounds)
  (params (NewVolume :type Physics%20Volume%20Object%20Reference)))

(event EventBeginPlay)

(event Collision|EventActorBeginOverlap
  (params (OtherActor :type Actor%20Object%20Reference)))

(event EventTick
  (params (DeltaSeconds :type Float%20%28single-precision%29))
  (Utilities|FlowControl|Sequence
    (:then_0
      ;[1 1 1] Animal Sounds while hovering.
      (if (Math|Boolean|Equal(Boolean) (Variables|/Game/SpaceRace/Components/HoverComponent.HoverComponent_C|GetHoverStatus (Variables|Default|GetHover)) true)
        (if (not (Audio|Components|Audio|IsPlaying (Variables|Default|GetAnimalSounds)))
          (Audio|Components|Audio|Play (Variables|Default|GetAnimalSounds) 0.0)
          (Audio|Components|Audio|FadeIn (Variables|Default|GetAnimalSounds) 5.0 0.5 0.0 :!class /Script/Engine.AudioComponent))
        (elif (Audio|Components|Audio|IsPlaying (Variables|Default|GetAnimalSounds))
          (Audio|Components|Audio|FadeOut (Variables|Default|GetAnimalSounds) 5.0 0.5 :!class /Script/Engine.AudioComponent))))
    (:then_1
      (if true
        _))))

(fn ConstructionScript)