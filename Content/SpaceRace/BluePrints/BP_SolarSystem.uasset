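; BP_SolarSystem is an animated solar system actor for SpaceRace, with a star and five coloured planets that moves across the screen.
; On BeginPlay, Timeline_0 drives the actor's location as an offset from its initial position.
; Each Tick rolls nested rotation-point components, scaled by DeltaSeconds, to spin the star and each planet.
; Separate orbital-path pivots share the base RotationSpeed plus per-planet offsets, so the planets orbit at different rates.
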(event EventTick
  (params (DeltaSeconds :type Float%20%28single-precision%29))
  (Utilities|FlowControl|Sequence
    (:then_0
      ;[1 1 1] Star's Rotation
      (Transformation|AddRelativeRotation (Variables|Default|GetRotationPoimt_Star) (* (Math|Rotator|MakeRotator (Variables|Default|GetRotation_Speed) 0.0 0.0) DeltaSeconds) false false))
    (:then_1
      ;[1 1 1] Rust Planet's Rotation and Orbit
      (Transformation|AddRelativeRotation (Variables|Default|GetRotationPoint_OrbitalPath_RustPlanet) (* (Math|Rotator|MakeRotator (+ (Variables|Default|GetRotation_Speed) 2e+01) 0.0 0.0) DeltaSeconds) false false)
      (Transformation|AddRelativeRotation (Variables|Default|GetRotationPoint_RustPlanet) (* (Math|Rotator|MakeRotator (Variables|Default|GetRotation_Speed) 0.0 0.0) DeltaSeconds) false false))
    (:then_2
      ;[1 1 1] Purple  Planet's Rotation and Orbit
      (Transformation|AddRelativeRotation (Variables|Default|GetRotationPoint_OrbitalPath_PurplePlanet) (* (Math|Rotator|MakeRotator (+ (Variables|Default|GetRotation_Speed) 15.0) 0.0 0.0) DeltaSeconds) false false)
      (Transformation|AddRelativeRotation (Variables|Default|GetRotationPoint_PurplePlanet) (* (Math|Rotator|MakeRotator (Variables|Default|GetRotation_Speed) 0.0 0.0) DeltaSeconds) false false))
    (:then_3
      ;[1 1 1] Green  Planet's Rotation and Orbit
      (Transformation|AddRelativeRotation (Variables|Default|GetRotationPoint_OrbitalPath_GreenPlanet) (* (Math|Rotator|MakeRotator (+ (Variables|Default|GetRotation_Speed) 1e+01) 0.0 0.0) DeltaSeconds) false false)
      (Transformation|AddRelativeRotation (Variables|Default|GetRotationPoint_GreenPlanet) (* (Math|Rotator|MakeRotator (Variables|Default|GetRotation_Speed) 0.0 0.0) DeltaSeconds) false false))
    (:then_4
      ;[1 1 1] Brown  Planet's Rotation and Orbit
      (Transformation|AddRelativeRotation (Variables|Default|GetRotationPoint_OrbitalPath_BrownPlanet) (* (Math|Rotator|MakeRotator (+ (Variables|Default|GetRotation_Speed) 5.0) 0.0 0.0) DeltaSeconds) false false)
      (Transformation|AddRelativeRotation (Variables|Default|GetRotationPoint_BrownPlanet) (* (Math|Rotator|MakeRotator (Variables|Default|GetRotation_Speed) 0.0 0.0) DeltaSeconds) false false))
    (:then_5
      ;[1 1 1] Blue  Planet's Rotation and Orbit
      (Transformation|AddRelativeRotation (Variables|Default|GetRotationPoint_OrbitalPath_BluePlanet) (* (Math|Rotator|MakeRotator (Variables|Default|GetRotation_Speed) 0.0 0.0) DeltaSeconds) false false)
      (Transformation|AddRelativeRotation (Variables|Default|GetRotationPoint_BluePlanet) (* (Math|Rotator|MakeRotator (Variables|Default|GetRotation_Speed) 0.0 0.0) DeltaSeconds) false false))))

(event EventBeginPlay
  ;[1 1 1] Solar System's Linear Movement Across the Screen
  (Variables|Default|SetActorInitialLocation (Transformation|GetActorLocation))
  (bind _movement (Timeline|Timeline_0 Play)
    (:Update
      (Transformation|SetActorLocation (+ _movement (Variables|Default|GetActorInitialLocation)) false false))))

(fn ConstructionScript)